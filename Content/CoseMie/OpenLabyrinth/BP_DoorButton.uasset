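; BP_DoorButton is an interactable button in the open labyrinth that opens its linked Door when the player presses E nearby.
; A box overlap with the player character enables pressing.
; The press fires once, triggers the character's Interact, then after a one-second delay turns the button light green and calls OpenDoor.
; The FloorGameManager reset event closes the door, restores the light material and re-arms the button.
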(event OnComponentBeginOverlap(Box)
  (params (OverlappedComponent :type Primitive%20Component%20Object%20Reference) (OtherActor :type Actor%20Object%20Reference) (OtherComp :type Primitive%20Component%20Object%20Reference) (OtherBodyIndex :type Integer) (bFromSweep :type Boolean) (SweepResult :type Hit%20Result%20Structure%20%28by%20ref%29))
  (Utilities|Casting|CastToBP_MyThirdPersonCharacterDoozy OtherActor)
  (Variables|Default|SetcanPressButton true))

(event OnComponentEndOverlap(Box)
  (params (OverlappedComponent :type Primitive%20Component%20Object%20Reference) (OtherActor :type Actor%20Object%20Reference) (OtherComp :type Primitive%20Component%20Object%20Reference) (OtherBodyIndex :type Integer))
  (Utilities|Casting|CastToBP_MyThirdPersonCharacterDoozy OtherActor)
  (Variables|Default|SetcanPressButton false))

(event Custom|HandleReset
  (Default|CloseDooronReset (Variables|Default|GetDoor))
  (Rendering|Material|SetMaterial (Variables|Default|GetCube2) 0 "/Game/CoseMie/OpenLabyrinth/M_ButtonLight.M_ButtonLight")
  (Utilities|FlowControl|DoOnce false) ; enters at Reset
)

(event EventBeginPlay
  (Input|EnableInput (Game|GetPlayerController 0))
  (EventDispatchers|BindEventtoResetGame (Variables|Default|GetFloorGameManager) (delegate Custom|HandleReset)))

(event Input|KeyboardEvents|E
  (params (Key :type Key%20Structure :default "None"))
  (:Pressed
    (if (Variables|Default|GetcanPressButton)
      (Utilities|FlowControl|DoOnce false
        (:Completed
          (bind _asbp_my_third_person_character_doozy (Utilities|Casting|CastToBP_MyThirdPersonCharacterDoozy (Game|GetPlayerCharacter 0)))
          (Default|Interact _asbp_my_third_person_character_doozy)
          (Utilities|FlowControl|Delay 1.0)
          (Rendering|Material|SetMaterial (Variables|Default|GetCube2) 0 "/Game/CoseMie/OpenLabyrinth/M_ButtonLightGreen.M_ButtonLightGreen")
          (Default|OpenDoor (Variables|Default|GetDoor)))))))

(fn ConstructionScript)