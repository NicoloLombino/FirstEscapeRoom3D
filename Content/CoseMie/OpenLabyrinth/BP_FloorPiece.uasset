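; BP_FloorPiece is a floor tile for a labyrinth minigame that is either safe or deadly, set by IsRightFloor.
; When BP_MyThirdPersonCharacter overlaps its Box, the Cube switches to one of two pulse materials.
; A wrong tile also calls the character's Death and, after a short delay, tells FloorManager to reset the game.
; Each tile binds to FloorManager's ResetGame event to restore its default material.
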(event OnComponentBeginOverlap(Box)
  (params (OverlappedComponent :type Primitive%20Component%20Object%20Reference) (OtherActor :type Actor%20Object%20Reference) (OtherComp :type Primitive%20Component%20Object%20Reference) (OtherBodyIndex :type Integer) (bFromSweep :type Boolean) (SweepResult :type Hit%20Result%20Structure%20%28by%20ref%29))
  (bind _cube (Variables|Default|GetCube))
  (bind _asbp_my_third_person_character (Utilities|Casting|CastToBP_MyThirdPersonCharacter OtherActor))
  (if (Variables|Default|GetisRightFloor)
    (Rendering|Material|SetMaterial _cube 0 "/Game/StarterContent/Materials/M_Tech_Hex_Tile_Pulse.M_Tech_Hex_Tile_Pulse")
    (else
      (Rendering|Material|SetMaterial _cube 0 "/Game/CoseMie/M_MyTech_Hex_Tile_Pulse.M_MyTech_Hex_Tile_Pulse")
      (Default|Death _asbp_my_third_person_character)
      (Utilities|FlowControl|Delay 1.8)
      (Default|ResetFloorGame (Variables|Default|GetFloorManager)))))

(event Custom|HandleResetFloor
  (Rendering|Material|SetMaterial (Variables|Default|GetCube) 0 "/Game/StarterContent/Materials/M_Tech_Hex_Tile.M_Tech_Hex_Tile"))

(event Collision|EventActorBeginOverlap
  (params (OtherActor :type Actor%20Object%20Reference)))

(event EventTick
  (params (DeltaSeconds :type Float%20%28single-precision%29)))

(event EventBeginPlay
  (EventDispatchers|BindEventtoResetGame (Variables|Default|GetFloorManager) (delegate Custom|HandleResetFloor)))

(fn ConstructionScript)