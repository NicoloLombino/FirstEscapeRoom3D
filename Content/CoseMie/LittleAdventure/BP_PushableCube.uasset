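; BP_PushableCube is a cube the adventure third-person character can push by holding E.
; Its Box overlap enables player input on the cube while that character is inside and disables it on exit.
; Pressing E without a torch starts the character's pushing state and attaches to its PushingTransform, keeping world transform.
; Releasing E ends pushing and detaches.
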(event OnComponentBeginOverlap(Box)
  (params (OverlappedComponent :type Primitive%20Component%20Object%20Reference) (OtherActor :type Actor%20Object%20Reference) (OtherComp :type Primitive%20Component%20Object%20Reference) (OtherBodyIndex :type Integer) (bFromSweep :type Boolean) (SweepResult :type Hit%20Result%20Structure%20%28by%20ref%29))
  (Utilities|Casting|CastToBP_MyThirdPersonCharacterAdventure OtherActor)
  (Input|EnableInput (Game|GetPlayerController 0)))

(event OnComponentEndOverlap(Box)
  (params (OverlappedComponent :type Primitive%20Component%20Object%20Reference) (OtherActor :type Actor%20Object%20Reference) (OtherComp :type Primitive%20Component%20Object%20Reference) (OtherBodyIndex :type Integer))
  (Utilities|Casting|CastToBP_MyThirdPersonCharacterAdventure OtherActor)
  (Input|DisableInput (Game|GetPlayerController 0)))

(event Input|KeyboardEvents|E
  (params (Key :type Key%20Structure :default "None"))
  (bind _returnvalue (Game|Player|GetPlayerPawn 0))
  (:Pressed
    (bind _asbp_my_third_person_character_adventure (Utilities|Casting|CastToBP_MyThirdPersonCharacterAdventure _returnvalue))
    (if (== (Variables|/Game/CoseMie/BP_MyThirdPersonCharacterAdventure.BP_MyThirdPersonCharacterAdventure_C|GetHasTorchValue _asbp_my_third_person_character_adventure) 0.0)
      (Default|GoPushing _asbp_my_third_person_character_adventure true)
      (Transformation|AttachComponentToComponent (Variables|/Game/CoseMie/BP_MyThirdPersonCharacterAdventure.BP_MyThirdPersonCharacterAdventure_C|GetPushingTransform _asbp_my_third_person_character_adventure) "None" "KeepWorld" "KeepWorld" "KeepWorld" true)))
  (:Released
    (bind _asbp_my_third_person_character_adventure_2 (Utilities|Casting|CastToBP_MyThirdPersonCharacterAdventure _returnvalue))
    (Default|GoPushing _asbp_my_third_person_character_adventure_2 false)
    (Transformation|DetachFromActor "KeepWorld" "KeepWorld" "KeepWorld")))

(fn ConstructionScript)