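; BP_AmbientTorch is a world torch the player can light when nearby.
; Overlapping its box toggles input for the adventure character, so pressing E works only inside it.
; E on an unlit torch requires the character's HasTorchValue to be full, then triggers an up or down torch action based on IsUpLight.
; TurnLight then shows the point light and particle effect; nothing here turns them off.
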(event OnComponentBeginOverlap(Box)
  (params (OverlappedComponent :type Primitive%20Component%20Object%20Reference) (OtherActor :type Actor%20Object%20Reference) (OtherComp :type Primitive%20Component%20Object%20Reference) (OtherBodyIndex :type Integer) (bFromSweep :type Boolean) (SweepResult :type Hit%20Result%20Structure%20%28by%20ref%29))
  (Utilities|Casting|CastToBP_MyThirdPersonCharacterAdventure OtherActor)
  (Input|EnableInput (Game|GetPlayerController 0)))

(event OnComponentEndOverlap(Box)
  (params (OverlappedComponent :type Primitive%20Component%20Object%20Reference) (OtherActor :type Actor%20Object%20Reference) (OtherComp :type Primitive%20Component%20Object%20Reference) (OtherBodyIndex :type Integer))
  (Utilities|Casting|CastToBP_MyThirdPersonCharacterAdventure OtherActor)
  (Input|DisableInput (Game|GetPlayerController 0)))

(event Custom|TurnLight
  (params (bNewVisibility :type Boolean))
  (Rendering|SetVisibility (Variables|Default|GetPointLight) bNewVisibility false)
  (Rendering|SetVisibility (Variables|Default|GetParticleSystem) bNewVisibility false))

(event EventBeginPlay)

(event Collision|EventActorBeginOverlap
  (params (OtherActor :type Actor%20Object%20Reference)))

(event EventTick
  (params (DeltaSeconds :type Float%20%28single-precision%29)))

(event Input|KeyboardEvents|E
  (params (Key :type Key%20Structure :default "None"))
  (:Pressed
    (if (not (Variables|/Script/Engine.SceneComponent|GetbVisible (Variables|Default|GetPointLight)))
      (bind _asbp_my_third_person_character_adventure (Utilities|Casting|CastToBP_MyThirdPersonCharacterAdventure (Game|Player|GetPlayerPawn 0)))
      (if (== (Variables|/Game/CoseMie/BP_MyThirdPersonCharacterAdventure.BP_MyThirdPersonCharacterAdventure_C|GetHasTorchValue _asbp_my_third_person_character_adventure) 1e+02)
        (if (Variables|Default|GetIsUpLight)
          (Default|DoTorchAction _asbp_my_third_person_character_adventure "UseTorchUp")
          (else
            (Default|DoTorchAction _asbp_my_third_person_character_adventure "UseTorchDown")))
        (CallFunction|TurnLight true)))))

(fn ConstructionScript)