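; BP_BallLVL3 is a physics ball for level 3 of a ball game that respawns after falling and can absorb other balls of its class.
; Tick watches for a drop below a height threshold, then after a delay teleports it to its BeginPlay location plus an offset and clears velocity.
; When flagged as main ball, Sphere1 overlaps set its scale slightly above the other ball's, swap its material and destroy that ball.
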(event OnComponentBeginOverlap(Sphere1)
  (params (OverlappedComponent :type Primitive%20Component%20Object%20Reference) (OtherActor :type Actor%20Object%20Reference) (OtherComp :type Primitive%20Component%20Object%20Reference) (OtherBodyIndex :type Integer) (bFromSweep :type Boolean) (SweepResult :type Hit%20Result%20Structure%20%28by%20ref%29))
  (bind _asbp_ball_lvl3 (Utilities|Casting|CastToBP_BallLVL3 OtherActor))
  (if (Variables|Default|GetisMainBall)
    (if (!= _asbp_ball_lvl3 self)
      (Transformation|SetRelativeScale3D (Variables|Default|GetSphere) (+ "0.100000,0.100000,0.100000" (Variables|/Script/Engine.SceneComponent|GetRelativeScale3D (Variables|BP_BallLVL3_C|GetSphere _asbp_ball_lvl3))))
      (Rendering|Material|SetMaterial (Variables|Default|GetSphere) 0 "/Game/StarterContent/Materials/M_Tech_Hex_Tile_Pulse.M_Tech_Hex_Tile_Pulse")
      (Actor|DestroyActor _asbp_ball_lvl3))))

(event Custom|Restart
  (Utilities|FlowControl|Delay 2.0)
  (Transformation|SetWorldLocation (Variables|Default|GetSphere) (+ (Variables|Default|GetStartLocation) (Variables|Default|GetHeightOnRestart)) false true)
  (Physics|SetPhysicsLinearVelocity (Variables|Default|GetSphere) "0, 0, 0" false "None"))

(event EventBeginPlay
  (Variables|Default|SetStartLocation (Transformation|GetWorldLocation (Variables|Default|GetSphere))))

(event EventTick
  (params (DeltaSeconds :type Float%20%28single-precision%29))
  (if (<= (.z (Transformation|GetWorldLocation (Variables|Default|GetSphere))) -2.5e+02)
    (CallFunction|Restart)))

(fn ConstructionScript)