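; BP_Ball is a ball that respawns after falling out of the level in Ball Adventure.
; It records the Sphere's starting location on BeginPlay and checks its height every Tick against a kill threshold.
; Falling below it calls Restart, which after a short Delay teleports the Sphere above its start and zeroes linear velocity, leaving angular velocity untouched.
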(event Custom|Restart
  (Utilities|FlowControl|Delay 2.0)
  (Transformation|SetWorldLocation (Variables|Default|GetSphere) (+ (Variables|Default|GetStartLocation) "0.000000,0.000000,200.000000") false true)
  (Physics|SetPhysicsLinearVelocity (Variables|Default|GetSphere) "0, 0, 0" false "None"))

(event EventBeginPlay
  (Variables|Default|SetStartLocation (Transformation|GetWorldLocation (Variables|Default|GetSphere))))

(event EventTick
  (params (DeltaSeconds :type Float%20%28single-precision%29))
  (if (<= (.z (Transformation|GetWorldLocation (Variables|Default|GetSphere))) -2.5e+02)
    (CallFunction|Restart)))

(fn ConstructionScript)