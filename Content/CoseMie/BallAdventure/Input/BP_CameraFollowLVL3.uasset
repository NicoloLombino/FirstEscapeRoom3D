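; Camera follow actor, apparently for level 3 of BallAdventure, that makes UpCamera the first player's view on BeginPlay.
; It also stores its own starting location as Offset.
; Logic to place UpCamera at the midpoint of Ball and Ball2 plus Offset exists but is disconnected.
; Tick is empty, so the graph never moves the camera.
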(event EventBeginPlay
  (Game|Player|SetViewTargetwithBlend (Game|GetPlayerController 0) (Variables|Default|GetUpCamera) 0.0 "VTBlend_Linear" 0.0 false)
  (Variables|Default|Setoffset (Transformation|GetActorLocation)))

(event EventTick
  (params (DeltaSeconds :type Float%20%28single-precision%29)))

(fn ConstructionScript)