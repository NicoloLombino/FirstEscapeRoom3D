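; BP_CameraFollow makes a camera follow the ball in the Ball Adventure game.
; On BeginPlay it sets player 0's view target to the UpCamera actor and stores its own actor location as the Offset.
; Each Tick it moves UpCamera to the ball sphere's world location plus that Offset, so only position follows, with no smoothing or rotation.
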(event EventBeginPlay
  (Game|Player|SetViewTargetwithBlend (Game|GetPlayerController 0) (Variables|Default|GetUpCamera) 0.0 "VTBlend_Linear" 0.0 false)
  (Variables|Default|Setoffset (Transformation|GetActorLocation)))

(event EventTick
  (params (DeltaSeconds :type Float%20%28single-precision%29))
  (Transformation|SetWorldLocation (Variables|/Script/Engine.Actor|GetRootComponent (Variables|Default|GetUpCamera)) (+ (Transformation|GetWorldLocation (Variables|/Game/CoseMie/BallAdventure/BP_Ball.BP_Ball_C|GetSphere (Variables|Default|GetBall))) (Variables|Default|Getoffset)) false false))

(fn ConstructionScript)