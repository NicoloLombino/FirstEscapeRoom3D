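; BP_RestartWall is a restart trigger for the ball adventure game that sends the ball back to its starting point.
; On BeginPlay it stores the world location of the referenced Ball's root component.
; When the Ball overlaps its Box, it waits a short delay, moves the Ball to that stored location without sweep, and prints the resulting position.
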(event OnComponentBeginOverlap(Box)
  (params (OverlappedComponent :type Primitive%20Component%20Object%20Reference) (OtherActor :type Actor%20Object%20Reference) (OtherComp :type Primitive%20Component%20Object%20Reference) (OtherBodyIndex :type Integer) (bFromSweep :type Boolean) (SweepResult :type Hit%20Result%20Structure%20%28by%20ref%29))
  (bind _ball (Variables|Default|GetBall))
  (if (== OtherActor _ball)
    (Utilities|FlowControl|Delay 2.0)
    (Transformation|SetWorldLocation (Variables|/Script/Engine.Actor|GetRootComponent _ball) (Variables|Default|GetStartPosition) false false)
    (Development|PrintString (Utilities|String|ToString(Vector) (Transformation|GetWorldLocation (Variables|/Script/Engine.Actor|GetRootComponent (Variables|Default|GetBall)))))))

(event EventBeginPlay
  (Variables|Default|SetStartPosition (Transformation|GetWorldLocation (Variables|/Script/Engine.Actor|GetRootComponent (Variables|Default|GetBall)))))

(fn ConstructionScript)