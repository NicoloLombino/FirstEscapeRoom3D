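; BP_BallFloor is the player-tilted floor for the Ball Adventure game.
; On BeginPlay it enables input for player 0, then after a short delay swaps the default Enhanced Input mapping context for the Ball Adventure one.
; Two move-floor input actions add roll and pitch to the Scene component's relative rotation, clamping each to plus or minus MaxAngle and keeping yaw at zero.
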(event Input|EnhancedActionEvents|EnhancedInputActionIA_MoveFloorX
  (params (ActionValue :type Float%20%28double-precision%29) (ElapsedSeconds :type Float%20%28double-precision%29) (TriggeredSeconds :type Float%20%28double-precision%29) (InputAction :type Input%20Action%20Object%20Reference :default "/Game/CoseMie/BallAdventure/Input/IA_MoveFloorX.IA_MoveFloorX"))
  (bind _scene (Variables|Default|GetScene))
  (bind _maxangle (Variables|Default|GetMaxAngle))
  (bind _relativerotation (Variables|/Script/Engine.SceneComponent|GetRelativeRotation _scene))
  (Transformation|AddRelativeRotation (Variables|Default|GetScene) (Math|Rotator|MakeRotator ActionValue 0.0 0.0) false false)
  (Transformation|SetRelativeRotation (Variables|Default|GetScene) (Math|Rotator|MakeRotator (Math|Float|Clamp(Float) (.roll _relativerotation) (* _maxangle -1.0) _maxangle) (.pitch _relativerotation) 0.0) false false))

(event Input|EnhancedActionEvents|EnhancedInputActionIA_MoveFloorY
  (params (ActionValue :type Float%20%28double-precision%29) (ElapsedSeconds :type Float%20%28double-precision%29) (TriggeredSeconds :type Float%20%28double-precision%29) (InputAction :type Input%20Action%20Object%20Reference :default "/Game/CoseMie/BallAdventure/Input/IA_MoveFloorY.IA_MoveFloorY"))
  (bind _scene (Variables|Default|GetScene))
  (bind _maxangle (Variables|Default|GetMaxAngle))
  (bind _relativerotation (Variables|/Script/Engine.SceneComponent|GetRelativeRotation _scene))
  (Transformation|AddRelativeRotation (Variables|Default|GetScene) (Math|Rotator|MakeRotator 0.0 ActionValue 0.0) false false)
  (Transformation|SetRelativeRotation (Variables|Default|GetScene) (Math|Rotator|MakeRotator (.roll _relativerotation) (Math|Float|Clamp(Float) (.pitch _relativerotation) (* _maxangle -1.0) _maxangle) 0.0) false false))

(event EventBeginPlay
  (bind _returnvalue (Game|GetPlayerController 0))
  (bind _returnvalue_2 (PlayerController|LocalPlayerSubsystems|GetEnhancedInputLocalPlayerSubsystem _returnvalue))
  (Input|EnableInput _returnvalue)
  (Utilities|FlowControl|Delay 0.2)
  (Input|AddMappingContext _returnvalue_2 "/Game/CoseMie/BallAdventure/Input/IMC_BallAdventureMap.IMC_BallAdventureMap" 0 "(bIgnoreAllPressedKeysUntilRelease=True,bForceImmediately=False,bNotifyUserSettings=False)")
  (Input|RemoveMappingContext _returnvalue_2 "/Game/ThirdPerson/Input/IMC_Default.IMC_Default" "(bIgnoreAllPressedKeysUntilRelease=True,bForceImmediately=False,bNotifyUserSettings=False)"))

(fn ConstructionScript)