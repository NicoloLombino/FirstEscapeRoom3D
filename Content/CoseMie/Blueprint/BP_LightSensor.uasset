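; BP_LightSensor is a blinking spotlight hazard that kills the third-person player character on contact with its sphere trigger.
; A looping timer started on BeginPlay drives a FlipFlop that toggles the SpotLight's visibility.
; Sphere overlap calls the character's Death, then after a delay spawns an explosion emitter at the sphere's location.
; The overlap never checks the light's state, so the trigger kills even while the light is hidden.
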(event OnComponentBeginOverlap(Sphere)
  (params (OverlappedComponent :type Primitive%20Component%20Object%20Reference) (OtherActor :type Actor%20Object%20Reference) (OtherComp :type Primitive%20Component%20Object%20Reference) (OtherBodyIndex :type Integer) (bFromSweep :type Boolean) (SweepResult :type Hit%20Result%20Structure%20%28by%20ref%29))
  (bind _asbp_third_person_character (Utilities|Casting|CastToBP_ThirdPersonCharacter OtherActor))
  (Variables|Default|SetPlayerLocation (Transformation|GetActorLocation (Game|GetPlayerController 0)))
  (Default|Death _asbp_third_person_character)
  (Utilities|FlowControl|Delay 5.0)
  (Effects|SpawnEmitteratLocation "/Game/StarterContent/Particles/P_Explosion.P_Explosion" (Transformation|GetWorldLocation (Variables|Default|GetSphere)) "0, 0, 0" "1.000000,1.000000,1.000000" false))

(event Custom|VisibilityLight
  (bind _isa (Utilities|FlowControl|FlipFlop)
    (:A
      _)
    (:B
      _))
  (Rendering|SetVisibility (Variables|Default|GetSpotLight) _isa false))

(event EventBeginPlay
  (Utilities|Time|SetTimerbyEvent (delegate Custom|VisibilityLight) (Variables|Default|GetLightTimer) true))

(fn ConstructionScript)