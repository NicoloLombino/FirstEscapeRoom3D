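; BP_Elevator is an elevator that responds to the third-person character entering or leaving its trigger box.
; Entering plays a timeline that shifts Cube1, the base, along Z, and leaving reverses it.
; That timeline's event tracks toggle StartMovement, which Tick polls to play or reverse a second timeline.
; The second timeline moves Cube vertically while spinning Scene two full turns in yaw, using start transforms cached on BeginPlay.
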(event OnComponentBeginOverlap(Box)
  (params (OverlappedComponent :type Primitive%20Component%20Object%20Reference) (OtherActor :type Actor%20Object%20Reference) (OtherComp :type Primitive%20Component%20Object%20Reference) (OtherBodyIndex :type Integer) (bFromSweep :type Boolean) (SweepResult :type Hit%20Result%20Structure%20%28by%20ref%29))
  (Utilities|Casting|CastToBP_ThirdPersonCharacter OtherActor)
  (bind _movement (Timeline|Timeline_0 Play)
    (:Update
      (Transformation|SetRelativeLocation (Variables|Default|GetCube1) (Math|Vector|MakeVector 0.0 0.0 (Math|Float|Lerp (Variables|Default|GetBaseStartPositionZ) (Variables|Default|GetBaseEndPositionZ) _movement)) false false))
    (:SetBoolTrue
      (Variables|Default|SetStartMovement true))
    (:SetBoolFalse
      (Variables|Default|SetStartMovement false))))

(event OnComponentEndOverlap(Box)
  (params (OverlappedComponent :type Primitive%20Component%20Object%20Reference) (OtherActor :type Actor%20Object%20Reference) (OtherComp :type Primitive%20Component%20Object%20Reference) (OtherBodyIndex :type Integer))
  (Utilities|Casting|CastToBP_ThirdPersonCharacter OtherActor)
  (bind _movement (Timeline|Timeline_0 Reverse)
    (:Update
      (Transformation|SetRelativeLocation (Variables|Default|GetCube1) (Math|Vector|MakeVector 0.0 0.0 (Math|Float|Lerp (Variables|Default|GetBaseStartPositionZ) (Variables|Default|GetBaseEndPositionZ) _movement)) false false))
    (:SetBoolTrue
      (Variables|Default|SetStartMovement true))
    (:SetBoolFalse
      (Variables|Default|SetStartMovement false))))

(event Custom|SetPositionBase
  (Variables|Default|SetBaseStartPositionZ (.z (Variables|/Script/Engine.SceneComponent|GetRelativeLocation (Variables|Default|GetCube1)))))

(event Custom|SetPositionElevator
  (bind _cube (Variables|Default|GetCube))
  (bind _relativelocation (Variables|/Script/Engine.SceneComponent|GetRelativeLocation _cube))
  (Variables|Default|SetStartPositionX (.x _relativelocation))
  (Variables|Default|SetStartPositionY (.y _relativelocation))
  (Variables|Default|SetStartPositionZ (.z _relativelocation)))

(event Custom|SetRotationElevator
  (Variables|Default|SetStartRotationZ (.yaw (Variables|/Script/Engine.SceneComponent|GetRelativeRotation (Variables|Default|GetScene))))
  (Variables|Default|SetEndRotationZ (+ (Variables|Default|GetStartRotationZ) 7.2e+02)))

(event EventTick
  (params (DeltaSeconds :type Float%20%28single-precision%29))
  (if (Variables|Default|GetStartMovement)
    (bind _newtrack_0 (Timeline|Timeline Play)
      (:Update
        (Transformation|SetRelativeLocation (Variables|Default|GetCube) (Math|Vector|MakeVector (Variables|Default|GetStartPositionX) (Variables|Default|GetStartPositionY) (Math|Float|Lerp (Variables|Default|GetStartPositionZ) (Variables|Default|GetEndPositionZ) _newtrack_0)) false false)
        (Transformation|SetRelativeRotation (Variables|Default|GetScene) (Math|Rotator|MakeRotator 0.0 0.0 (Math|Float|Lerp (Variables|Default|GetStartRotationZ) (Variables|Default|GetEndRotationZ) _newtrack_0)) false false)))
    (else
      (Timeline|Timeline Reverse))))

(event EventBeginPlay
  (CallFunction|SetPositionBase)
  (CallFunction|SetPositionElevator)
  (CallFunction|SetRotationElevator))

(fn ConstructionScript)