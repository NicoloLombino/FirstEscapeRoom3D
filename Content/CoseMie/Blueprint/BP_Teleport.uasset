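; Teleporter actor that moves BP_ThirdPersonCharacter to the Sphere1 component of its linked EndTeleport.
; Entering Sphere1 starts a one-shot timer of TimeToTeleport, and leaving clears it, so the character must stay inside until it fires.
; The Teleport event sets the character's location while toggling CanMove, and hides the destination sphere for a short delay without changing its collision.
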(event OnComponentBeginOverlap(Sphere1)
  (params (OverlappedComponent :type Primitive%20Component%20Object%20Reference) (OtherActor :type Actor%20Object%20Reference) (OtherComp :type Primitive%20Component%20Object%20Reference) (OtherBodyIndex :type Integer) (bFromSweep :type Boolean) (SweepResult :type Hit%20Result%20Structure%20%28by%20ref%29))
  (bind _asbp_third_person_character (Utilities|Casting|CastToBP_ThirdPersonCharacter OtherActor))
  (bind _returnvalue (Utilities|Time|SetTimerbyEvent (delegate Custom|Teleport) (Variables|Default|GetTimeToTeleport))))

(event OnComponentEndOverlap(Sphere1)
  (params (OverlappedComponent :type Primitive%20Component%20Object%20Reference) (OtherActor :type Actor%20Object%20Reference) (OtherComp :type Primitive%20Component%20Object%20Reference) (OtherBodyIndex :type Integer))
  (Utilities|Casting|CastToBP_ThirdPersonCharacter OtherActor)
  (Utilities|Time|ClearandInvalidateTimerbyHandle (stale OnComponentBeginOverlap(Sphere1) _returnvalue)))

(event Custom|Teleport
  (bind _endteleport (Variables|Default|GetEndTeleport))
  (bind _sphere1 (Variables|BP_Teleport_C|GetSphere1 _endteleport))
  (Rendering|SetVisibility _sphere1 false false)
  (Variables|/Game/ThirdPerson/Blueprints/BP_ThirdPersonCharacter.BP_ThirdPersonCharacter_C|SetCanMove (stale OnComponentBeginOverlap(Sphere1) _asbp_third_person_character) false)
  (Transformation|SetActorLocation (stale OnComponentBeginOverlap(Sphere1) _asbp_third_person_character) (Transformation|GetWorldLocation (Variables|BP_Teleport_C|GetSphere1 _endteleport)) false false)
  (Variables|/Game/ThirdPerson/Blueprints/BP_ThirdPersonCharacter.BP_ThirdPersonCharacter_C|SetCanMove (stale OnComponentBeginOverlap(Sphere1) _asbp_third_person_character) true)
  (Utilities|FlowControl|Delay 3.0)
  (Rendering|SetVisibility _sphere1 true false))

(event EventBeginPlay)

(event Collision|EventActorBeginOverlap
  (params (OtherActor :type Actor%20Object%20Reference)))

(event EventTick
  (params (DeltaSeconds :type Float%20%28single-precision%29)))

(fn ConstructionScript)