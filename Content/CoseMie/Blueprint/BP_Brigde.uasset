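; BP_Brigde is a bridge actor that rotates by a set increment whenever its MoveBridge event fires.
; The event stores the scene component's current relative rotation and adds MovementIncrement to compute the end rotation.
; A timeline's Movement track drives a rotator lerp between the two, then clears IsMoving when it finishes.
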(event Custom|MoveBridge
  (bind _movementincrement (Variables|Default|GetMovementIncrement))
  (Variables|Default|SetStartPosition (Variables|/Script/Engine.SceneComponent|GetRelativeRotation (Variables|Default|GetScene)))
  (Variables|Default|SetEndPosition (Math|Rotator|MakeRotator (+ (.roll (Variables|Default|GetStartPosition)) (.roll _movementincrement)) (+ (.pitch (Variables|Default|GetStartPosition)) (.pitch _movementincrement)) (+ (.yaw (Variables|Default|GetStartPosition)) (.yaw _movementincrement))))
  (bind _movement (Timeline|Timeline PlayFromStart)
    (:Update
      (Transformation|SetRelativeRotation (Variables|Default|GetScene) (Math|Rotator|Lerp(Rotator) (Variables|Default|GetStartPosition) (Variables|Default|GetEndPosition) _movement) false false))
    (:Finished
      (Variables|Default|SetIsMoving false))))

(fn ConstructionScript)