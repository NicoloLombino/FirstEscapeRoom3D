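; Coin-gated door that opens once its coin count, raised through AddCoin, reaches the required amount.
; The count is checked at BeginPlay and when the third-person character enters the trigger box, which also reveals a "coins/required" text until exit.
; Opening hides the text, turns the light green, then after a delay a timeline either slides the cube or rotates the scene pivot, destroying the light when finished.
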(event OnComponentBeginOverlap(Box)
  (params (OverlappedComponent :type Primitive%20Component%20Object%20Reference) (OtherActor :type Actor%20Object%20Reference) (OtherComp :type Primitive%20Component%20Object%20Reference) (OtherBodyIndex :type Integer) (bFromSweep :type Boolean) (SweepResult :type Hit%20Result%20Structure%20%28by%20ref%29))
  (bind _coins (Variables|Default|GetCoins))
  (bind _textrender (Variables|Default|GetTextRender))
  (bind _coinstoopen (Variables|Default|GetCoinsToOpen))
  (Utilities|Casting|CastToBP_ThirdPersonCharacter OtherActor)
  (Development|SetHiddeninGame _textrender false false)
  (Rendering|Components|TextRender|SetText _textrender (Utilities|Text|FormatText "{coins}/{coinsToOpen}" _coins _coinstoopen))
  (if (>= _coins _coinstoopen)
    (CallFunction|OpenDoor)))

(event OnComponentEndOverlap(Box)
  (params (OverlappedComponent :type Primitive%20Component%20Object%20Reference) (OtherActor :type Actor%20Object%20Reference) (OtherComp :type Primitive%20Component%20Object%20Reference) (OtherBodyIndex :type Integer))
  (Utilities|Casting|CastToBP_ThirdPersonCharacter OtherActor)
  (Development|SetHiddeninGame (Variables|Default|GetTextRender) true false))

(event Custom|OpenDoor
  (Development|SetHiddeninGame (Variables|Default|GetTextRender) true false)
  (Rendering|Components|Light|SetLightColor (Variables|Default|GetRectLight) "(R=0.000000,G=1.000000,B=0.008607,A=1.000000)" true)
  (Utilities|FlowControl|Delay 1.0)
  (bind _movement (Timeline|Timeline Play)
    (:Update
      (if (Variables|Default|GetLocationMovement)
        (Transformation|SetRelativeLocation (Variables|Default|GetCube) (Math|Vector|Lerp(Vector) (Variables|Default|GetStartLocation) (Variables|Default|GetEndLocation) _movement) false false)
        (else
          (Transformation|SetRelativeRotation (Variables|Default|GetScene) (Math|Rotator|Lerp(Rotator) (Variables|Default|GetStartRotation) (Variables|Default|GetEndRotation) _movement) false false))))
    (:Finished
      (Components|DestroyComponent (Variables|Default|GetRectLight)))))

(event Custom|AddCoin
  (Math|Integer|IncrementInt (Variables|Default|GetCoins)))

(event EventBeginPlay
  (bind _coins (Variables|Default|GetCoins))
  (bind _coinstoopen (Variables|Default|GetCoinsToOpen))
  (Variables|Default|SetStartLocation (Variables|/Script/Engine.SceneComponent|GetRelativeLocation (Variables|Default|GetCube)))
  (Variables|Default|SetStartRotation (Variables|/Script/Engine.SceneComponent|GetRelativeRotation (Variables|Default|GetScene)))
  (Rendering|Components|TextRender|SetText (Variables|Default|GetTextRender) (Utilities|Text|FormatText "{coins}/{coinsToOpen}" _coins _coinstoopen))
  (if (>= _coins _coinstoopen)
    (CallFunction|OpenDoor)))

(fn ConstructionScript)