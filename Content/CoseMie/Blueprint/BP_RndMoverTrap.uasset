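; BP_RndMoverTrap moves a referenced Trap in random grid steps on X and Y, starting at BeginPlay.
; GetRandomDirecion rolls -1, 0 or 1 per axis, immediately rerolling if the running step count would reach its min or max limit.
; A valid roll offsets the Trap's root by MovemenSize, then calls itself again after a MoveTime delay.
; Debug prints remain, and a looping-timer alternative is left unconnected.
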(event Custom|DoMovement
  (CallFunction|GetRandomDirecion))

(event Custom|GetRandomDirecion
  (bind _returnvalue (Class|KismetMathLibrary|RandomInteger64inRange -1 1))
  (bind _movemensize (Variables|Default|GetMovemenSize))
  (Variables|Default|SetTempX (Math|Conversions|ToInteger(Byte) _returnvalue))
  (Variables|Default|SetTempY (Math|Conversions|ToInteger(Byte) _returnvalue))
  (if (or (or (<= (+ (Variables|Default|GetTempX) (Variables|Default|GetMoveCountX)) (Variables|Default|GetMoveCountXMin)) (>= (+ (Variables|Default|GetTempX) (Variables|Default|GetMoveCountX)) (Variables|Default|GetMoveCountXMax))) (or (<= (+ (Variables|Default|GetTempY) (Variables|Default|GetMoveCountY)) (Variables|Default|GetMoveCountYMin)) (>= (+ (Variables|Default|GetTempY) (Variables|Default|GetMoveCountY)) (Variables|Default|GetMoveCountYMax))))
    (CallFunction|GetRandomDirecion)
    (Development|PrintString "OUT")
    (else
      (Variables|Default|SetRndDirectionX (Variables|Default|GetTempX))
      (Variables|Default|SetRndDirectionY (Variables|Default|GetTempY))
      (Variables|Default|SetMoveCountX (+ (Variables|Default|GetTempX) (Variables|Default|GetMoveCountX)))
      (Variables|Default|SetMoveCountY (+ (Variables|Default|GetTempY) (Variables|Default|GetMoveCountY)))
      (Transformation|AddWorldOffset (Variables|/Script/Engine.Actor|GetRootComponent (Variables|Default|GetTrap)) (Math|Vector|MakeVector (* (Variables|Default|GetRndDirectionX) _movemensize) (* (Variables|Default|GetRndDirectionY) _movemensize) 0.0) false false)
      (Development|PrintString (Utilities|String|ToString(Text) (Utilities|Text|FormatText "{a}--{b}--{c}" (Variables|Default|GetRndDirectionX) (Variables|Default|GetRndDirectionY))))
      (Utilities|FlowControl|Delay (Variables|Default|GetMoveTime))
      (CallFunction|GetRandomDirecion))))

(event EventBeginPlay
  (CallFunction|GetRandomDirecion))

(fn ConstructionScript)