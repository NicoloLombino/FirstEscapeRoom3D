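; BP_TimerLight is a spotlight actor that flashes on and off in randomly chosen colors.
; At BeginPlay it starts a looping timer whose interval is picked once at random between the configured minimum and maximum.
; Each tick of that timer shows the light in a random color from the Colors array, then hides it after a newly randomized delay within the same range.
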(event Custom|ActiveLight
  (bind _spotlight (Variables|Default|GetSpotLight))
  (Rendering|SetVisibility _spotlight true false)
  (Rendering|Components|Light|SetLightColor _spotlight (Math|Conversions|ToLinearColor(Color) (.OutItem (Utilities|Array|Random (Variables|Default|GetColors)))) true)
  (Utilities|FlowControl|Delay (Math|Random|RandomFloatinRange (Variables|Default|GetTimerMIn) (Variables|Default|GetTimerMax)))
  (Rendering|SetVisibility (Variables|Default|GetSpotLight) false false))

(event EventBeginPlay
  (Utilities|Time|SetTimerbyEvent (delegate Custom|ActiveLight) (Math|Random|RandomFloatinRange (Variables|Default|GetTimerMIn) (Variables|Default|GetTimerMax)) true))

(fn ConstructionScript)